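; Projectile Blueprint with a static mesh and a projectile movement component, set moving when play begins.
; BeginPlay deactivates the movement component, then calls Launch with a fixed speed and direction.
; Launch sets initial and maximum speed, zeroes the mesh's world rotation and reactivates movement.
; The direction argument is unused, as its rotation-from-vector node is left unconnected.
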(event EventBeginPlay
  (Components|Activation|SetActive (Variables|Default|GetProjectileMovement) false false)
  (CallFunction|Launch 1e+02 "1.000000,0.000000,0.000000"))

(fn ConstructionScript)

(fn Launch
  (params (Speed :type Float%20%28double-precision%29) (Dir :type Vector))
  (bind _projectilemovement (Variables|Default|GetProjectileMovement))
  (Variables|/Script/Engine.ProjectileMovementComponent|SetMaxSpeed _projectilemovement Speed)
  (Variables|/Script/Engine.ProjectileMovementComponent|SetInitialSpeed _projectilemovement Speed)
  (Transformation|SetWorldRotation (Variables|Default|GetStaticMesh) "0, 0, 0" false false)
  (Components|Activation|SetActive _projectilemovement true false))