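; BP_Health tracks an owner's health, starting CurrentHealth at MaxHealth on BeginPlay.
; ApplyDamage subtracts damage within a zero-to-max clamp, calls OnDeath at zero or OnDamage otherwise, and returns the new health with a dead flag.
; Death has no latch, so further damage at zero calls OnDeath again, and GetHealth exposes the current value.
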(event EventBeginPlay
  (Variables|Default|SetCurrentHealth (Variables|Default|GetMaxHealth)))

(fn ApplyDamage
  (params (Damage :type Float%20%28double-precision%29))
  (bind _output_get (Variables|Default|SetCurrentHealth (Math|Float|Clamp(Float) (- (Variables|Default|GetCurrentHealth) Damage) 0.0 (Variables|Default|GetMaxHealth))))
  (if (<= _output_get 0.0)
    (Default|CallOnDeath)
    (else
      (Default|CallOnDamage)))
  (return (<= _output_get 0.0) _output_get))

(fn GetHealth
  (return (Variables|Default|GetCurrentHealth)))