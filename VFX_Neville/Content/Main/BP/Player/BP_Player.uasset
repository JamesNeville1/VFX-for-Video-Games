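; Player character with move and look input plus a held life-transmute ability that drains enemies to heal teammates.
; While held, a looping timer sphere-traces nearby pawns, banking life from enemy dummies and spending it on team dummies.
; Each tick aims pre-spawned pools of five give and five take Niagara beams at those targets.
; BeginPlay also pre-spawns inactive effects from a data-driven chart, including the ability's toggled effect.
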(event Custom|Life%20Steal%20Main
  (bind _capsulecomponent (Variables|Collision|GetCapsuleComponent))
  (bind _returnvalue (Transformation|GetWorldLocation _capsulecomponent))
  (bind _outhits (Collision|MultiSphereTraceForObjects _returnvalue _returnvalue (Variables|LifeStealMechanic|GetLifeStealRangeRadius) (Utilities|Array|MakeArray "ObjectTypeQuery3") false 0 "ForDuration" true "(R=1.000000,G=0.000000,B=0.000000,A=1.000000)" "(R=0.000000,G=1.000000,B=0.000000,A=1.000000)" 0.2))
  (Utilities|Array|Clear (Variables|LifeStealMechanic|GetTeamToHeal))
  (Utilities|Array|Clear (Variables|LifeStealMechanic|GetEnemiesToTakeFrom))
  (for _array_element _outhits
    (if (== (Utilities|GetClass (.HitActor (Collision|BreakHitResult _array_element))) "/Game/Main/BP/BP_Dummy_Enemy.BP_Dummy_Enemy_C")
      (bind _actor_out (|LifeStealLogic (.HitActor (Collision|BreakHitResult _array_element))))
      (Utilities|Array|Add (Variables|LifeStealMechanic|GetEnemiesToTakeFrom) _actor_out)
      (elif (== (Utilities|GetClass (.HitActor (Collision|BreakHitResult _array_element))) "/Game/Main/BP/BP_Dummy_Team.BP_Dummy_Team_C")
        (bind _actor_out_2 (|LifeGiveLogic (.HitActor (Collision|BreakHitResult _array_element))))
        (Utilities|Array|Add (Variables|LifeStealMechanic|GetTeamToHeal) _actor_out_2))))
  (CallFunction|BeamSetup (Variables|LifeStealMechanic|GetTeamToHeal) (Variables|LifeStealMechanic|GetLifeBeams))
  (CallFunction|BeamSetup (Variables|LifeStealMechanic|GetEnemiesToTakeFrom) (Variables|LifeStealMechanic|GetLifeStealBeams)))

(event EventIAMoveT
  (params (in :type Vector%202D%20Structure))
  (bind (_x _y) (Math|Vector2D|BreakVector2D in))
  (bind _springarm (Variables|Default|GetSpringArm))
  (Pawn|Input|AddMovementInput (Math|Vector|GetForwardVector _springarm) _x false)
  (Pawn|Input|AddMovementInput (Math|Vector|GetRightVector _springarm) _y false))

(event EventIALookT
  (params (in :type Vector%202D%20Structure))
  (bind (_x _y) (Math|Vector2D|BreakVector2D in))
  (Pawn|Input|AddControllerYawInput (* _x 1.0))
  (Transformation|SetRelativeRotation (Variables|Default|GetSpringArm) (Math|Rotator|MakeRotator 0.0 (Math|Float|Clamp(Float) (+ (.pitch (Variables|/Script/Engine.SceneComponent|GetRelativeRotation (Variables|Default|GetSpringArm))) _y) (Variables|Default|GetLookPitchMin) (Variables|Default|GetLookPitchMax)) 0.0) false false))

(event EventBeginPlay
  (|EffectChartSetup)
  (|LifeTransmuteBeamCreate))

(event EventIALifeStealAbilityS
  (Components|Activation|SetActive (.Value (Utilities|Map|Find (Variables|Default|GetEffectChart) "NewEnumerator0")) true true)
  (bind _returnvalue (Utilities|Time|SetTimerbyEvent (delegate Custom|Life%20Steal%20Main) 0.2 true))
  (Variables|LifeStealMechanic|SetLifeStealLogicLoop _returnvalue))

(event EventIALifeStealAbilityE
  (Components|Activation|SetActive (.Value (Utilities|Map|Find (Variables|Default|GetEffectChart) "NewEnumerator0")) false true)
  (Utilities|Time|ClearandInvalidateTimerbyHandle (Variables|LifeStealMechanic|GetLifeStealLogicLoop))
  (CallFunction|TurnOffAllBeams))

(event EventIALifeStealAbilityT)

(fn ConstructionScript)

(fn SummonPooledEffect
  (params (id :type E_LifeTransmuteBeamID%20Enum :default "NewEnumerator0")))

(fn BeamSetup
  (params (Dummy :type Array%20of%20Actor%20Object%20References) (Niagara%20Systems :type Array%20of%20Niagara%20Component%20Object%20References))
  (for _index (range 0 4)
    (Utilities|IsValid (Utilities|Array|Get(acopy) Dummy _index)
      (:Is%20Valid
        (Components|Activation|SetActive (Utilities|Array|Get(acopy) Niagara%20Systems _index) true true)
        (Niagara|SetNiagaraVariable(Vector3) (Utilities|Array|Get(acopy) Niagara%20Systems _index) "Beam End" (+ (Transformation|GetActorLocation (Utilities|Array|Get(acopy) Dummy _index)) "0.000000,0.000000,80.000000")))
      (:Is%20Not%20Valid
        (Components|Activation|SetActive (Utilities|Array|Get(acopy) Niagara%20Systems _index) false true)))))

(fn TurnOffAllBeams
  (for _array_element (Variables|LifeStealMechanic|GetLifeBeams)
    (Components|Activation|SetActive _array_element false true))
  (for _array_element_2 (Variables|LifeStealMechanic|GetLifeStealBeams)
    (Components|Activation|SetActive _array_element_2 false true)))