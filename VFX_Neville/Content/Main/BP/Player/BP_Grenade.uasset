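; Healing grenade projectile that gives life to team dummies and destroys itself on contact.
; Sphere overlap with a BP_Dummy_Team sends it a delayed give-life message and a health effect message, then spawns the life burst Niagara system.
; Other overlaps and any hit share a miss path with a debug print and a hit-nothing burst.
; Both paths unhide the Trail just before destroying the actor.
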(event OnComponentBeginOverlap(Sphere)
  (params (OverlappedComponent :type Primitive%20Component%20Object%20Reference) (OtherActor :type Actor%20Object%20Reference) (OtherComp :type Primitive%20Component%20Object%20Reference) (OtherBodyIndex :type Integer) (bFromSweep :type Boolean) (SweepResult :type Hit%20Result%20Structure%20%28by%20ref%29))
  (if (== (Utilities|GetClass OtherActor) "/Game/Main/BP/BP_Dummy_Team.BP_Dummy_Team_C")
    (Class|BPIDummy|GiveLifeDelayed(Message) OtherActor 6.0 (Variables|Default|GetGive))
    (Class|BPIDummy|HealthGrenadeEffect(Message) OtherActor)
    (Niagara|SpawnSystematLocation "/Game/Main/VFX/Main/HealthGrenade/NS_LifeGrenadeBurst.NS_LifeGrenadeBurst" (Transformation|GetWorldLocation (Variables|Default|GetSphere)))
    (else
      (Development|PrintString "Hello")
      (Niagara|SpawnSystematLocation "/Game/Main/VFX/Main/HealthGrenade/NS_LifeGrenadeBurstHitNothing.NS_LifeGrenadeBurstHitNothing" (Transformation|GetWorldLocation (Variables|Default|GetSphere)))))
  (Development|SetHiddeninGame (Variables|Default|GetTrail) false false)
  (Actor|DestroyActor))

(event OnComponentHit(Sphere)
  (params (HitComponent :type Primitive%20Component%20Object%20Reference) (OtherActor :type Actor%20Object%20Reference) (OtherComp :type Primitive%20Component%20Object%20Reference) (NormalImpulse :type Vector :default "0, 0, 0") (Hit :type Hit%20Result%20Structure%20%28by%20ref%29))
  (Development|PrintString "Hello")
  (Niagara|SpawnSystematLocation "/Game/Main/VFX/Main/HealthGrenade/NS_LifeGrenadeBurstHitNothing.NS_LifeGrenadeBurstHitNothing" (Transformation|GetWorldLocation (Variables|Default|GetSphere)))
  (Development|SetHiddeninGame (Variables|Default|GetTrail) false false)
  (Actor|DestroyActor))

(fn ConstructionScript)