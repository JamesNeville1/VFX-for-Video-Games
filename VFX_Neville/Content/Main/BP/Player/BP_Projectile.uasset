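; Player projectile actor that explodes on contact, dealing area damage to dummy enemies.
; Sphere overlap and hit events share one path that runs a zero-length Pawn-profile sphere trace at the explosion radius.
; Each hit actor whose class is exactly BP_Dummy_Enemy receives Damage through TakeLifeMessage, then the projectile destroys itself.
; The Destroyed event spawns the molten explosion Niagara effect at the sphere's location.
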(event OnComponentBeginOverlap(Sphere)
  (params (OverlappedComponent :type Primitive%20Component%20Object%20Reference) (OtherActor :type Actor%20Object%20Reference) (OtherComp :type Primitive%20Component%20Object%20Reference) (OtherBodyIndex :type Integer) (bFromSweep :type Boolean) (SweepResult :type Hit%20Result%20Structure%20%28by%20ref%29))
  (bind _sphere (Variables|Default|GetSphere))
  (bind _returnvalue (Transformation|GetWorldLocation _sphere))
  (bind _outhits (Class|KismetSystemLibrary|SphereTraceMultibyProfile _returnvalue _returnvalue (Variables|Default|GetExplosionRadius) "Pawn" false 0 "None" true))
  (for _array_element _outhits
    (if (== (Utilities|GetClass (.HitActor (Collision|BreakHitResult _array_element))) "/Game/Main/BP/BP_Dummy_Enemy.BP_Dummy_Enemy_C")
      (Class|BPIDummy|TakeLife(Message) (.HitActor (Collision|BreakHitResult _array_element)) (Variables|Default|GetDamage))))
  (Actor|DestroyActor))

(event OnComponentHit(Sphere)
  (params (HitComponent :type Primitive%20Component%20Object%20Reference) (OtherActor :type Actor%20Object%20Reference) (OtherComp :type Primitive%20Component%20Object%20Reference) (NormalImpulse :type Vector :default "0, 0, 0") (Hit :type Hit%20Result%20Structure%20%28by%20ref%29))
  (bind _sphere (Variables|Default|GetSphere))
  (bind _returnvalue (Transformation|GetWorldLocation _sphere))
  (bind _outhits (Class|KismetSystemLibrary|SphereTraceMultibyProfile _returnvalue _returnvalue (Variables|Default|GetExplosionRadius) "Pawn" false 0 "None" true))
  (for _array_element _outhits
    (if (== (Utilities|GetClass (.HitActor (Collision|BreakHitResult _array_element))) "/Game/Main/BP/BP_Dummy_Enemy.BP_Dummy_Enemy_C")
      (Class|BPIDummy|TakeLife(Message) (.HitActor (Collision|BreakHitResult _array_element)) (Variables|Default|GetDamage))))
  (Actor|DestroyActor))

(event EventDestroyed
  (Niagara|SpawnSystematLocation "/Game/Main/VFX/Main/MoltenProjectile/NS_MoltenDeathExplode.NS_MoltenDeathExplode" (Transformation|GetWorldLocation (Variables|Default|GetSphere))))

(event EventBeginPlay)

(fn ConstructionScript)