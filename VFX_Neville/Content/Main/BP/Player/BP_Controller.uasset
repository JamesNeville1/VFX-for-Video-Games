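; Player controller that receives Enhanced Input and relays it to the player character, covering movement, look, shooting, life steal and life grenade.
; It adds the IMC_Player mapping context on BeginPlay.
; Each input action forwards its trigger, start or completion phase as a message to player character 0.
; It holds no gameplay logic itself, leaving the response to the character.
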(event Input|EnhancedActionEvents|EnhancedInputActionIA_LifeGrenade
  (params (ActionValue :type Boolean) (ElapsedSeconds :type Float%20%28double-precision%29) (TriggeredSeconds :type Float%20%28double-precision%29) (InputAction :type Input%20Action%20Object%20Reference :default "/Game/Main/BP/Player/IA_LifeGrenade.IA_LifeGrenade"))
  (:Started
    (Class|BPIPlayerInput|IALifeGrenadeS(Message) (Game|GetPlayerCharacter 0))))

(event Input|EnhancedActionEvents|EnhancedInputActionIA_Shoot
  (params (ActionValue :type Boolean) (ElapsedSeconds :type Float%20%28double-precision%29) (TriggeredSeconds :type Float%20%28double-precision%29) (InputAction :type Input%20Action%20Object%20Reference :default "/Game/Main/BP/Player/IA_Shoot.IA_Shoot"))
  (bind _returnvalue (Game|GetPlayerCharacter 0))
  (:Started
    (Class|BPIPlayerInput|IAShootS(Message) _returnvalue))
  (:Completed
    (Class|BPIPlayerInput|IAShootE(Message) _returnvalue)))

(event Input|EnhancedActionEvents|EnhancedInputActionIA_Move
  (params (ActionValue :type Vector%202D%20Structure) (ElapsedSeconds :type Float%20%28double-precision%29) (TriggeredSeconds :type Float%20%28double-precision%29) (InputAction :type Input%20Action%20Object%20Reference :default "/Game/Main/BP/Player/IA_Move.IA_Move"))
  (Class|BPIPlayerInput|IAMoveT(Message) (Game|GetPlayerCharacter 0) ActionValue))

(event Input|EnhancedActionEvents|EnhancedInputActionIA_Look
  (params (ActionValue :type Vector%202D%20Structure) (ElapsedSeconds :type Float%20%28double-precision%29) (TriggeredSeconds :type Float%20%28double-precision%29) (InputAction :type Input%20Action%20Object%20Reference :default "/Game/Main/BP/Player/IA_Look.IA_Look"))
  (Class|BPIPlayerInput|IALookT(Message) (Game|GetPlayerCharacter 0) ActionValue))

(event Input|EnhancedActionEvents|EnhancedInputActionIA_LifeStealAbility
  (params (ActionValue :type Boolean) (ElapsedSeconds :type Float%20%28double-precision%29) (TriggeredSeconds :type Float%20%28double-precision%29) (InputAction :type Input%20Action%20Object%20Reference :default "/Game/Main/BP/Player/IA_LifeStealAbility.IA_LifeStealAbility"))
  (bind _returnvalue (Game|GetPlayerCharacter 0))
  (:Triggered
    (Class|BPIPlayerInput|IALifeStealAbilityT(Message) _returnvalue))
  (:Started
    (Class|BPIPlayerInput|IALifeStealAbilityS(Message) _returnvalue))
  (:Completed
    (Class|BPIPlayerInput|IALifeStealAbilityE(Message) _returnvalue)))

(event EventBeginPlay
  (Input|AddMappingContext (PlayerController|LocalPlayerSubsystems|GetEnhancedInputLocalPlayerSubsystem self) "/Game/Main/BP/Player/IMC_Player.IMC_Player" 0 "(bIgnoreAllPressedKeysUntilRelease=True,bForceImmediately=False,bNotifyUserSettings=False)"))

(fn ConstructionScript)