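; BP_Dummy is a damageable, healable target actor with a health widget that turns to face the player camera each tick.
; A BPHealth component drives it: damage events refresh the widget's normalized health, and death disables mesh collision.
; Give Life heals by applying negative damage and spawns a Niagara effect, optionally after a timer, while Take Life applies damage.
; An empty ChildBeginPlay hook runs after setup for child Blueprints.
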(event Custom|On%20Give%20Life%20Delayed%20Finished
  (CallFunction|GiveLife (stale EventGiveLifeDelayed Give)))

(event Custom|OnDeath_Event
  (Collision|SetCollisionEnabled (Variables|Default|GetStaticMesh) "NoCollision"))

(event Custom|OnDamage_Event
  (bind _out (Default|GetNormalizedHealth (Variables|Default|GetBP_Health)))
  (Class|BPIUI|AdjustHealth(Message) (UserInterface|GetWidget (Variables|Default|GetWidget)) _out))

(event Custom|Child%20BeginPlay)

(event EventHealthGrenadeEffect
  (Niagara|SpawnSystematLocation "/Game/Main/VFX/Main/HealthGrenade/NS_LifeHealRing.NS_LifeHealRing" (Transformation|GetWorldLocation (Variables|Default|GetStaticMesh))))

(event EventGiveLifeDelayed
  (params (Delay :type Float%20%28double-precision%29) (Give :type Float%20%28double-precision%29))
  (Utilities|Time|SetTimerbyEvent (delegate Custom|On%20Give%20Life%20Delayed%20Finished) Delay))

(event EventTick
  (params (DeltaSeconds :type Float%20%28single-precision%29))
  (Transformation|SetWorldRotation (Variables|Default|GetWidget) (Math|Rotator|FindLookatRotation (Transformation|GetWorldLocation (Variables|Default|GetWidget)) (Transformation|GetWorldLocation (Variables|/Script/Engine.PlayerCameraManager|GetTransformComponent (Game|GetPlayerCameraManager 0)))) false false))

(event EventBeginPlay
  (bind _bp_health (Variables|Default|GetBP_Health))
  (EventDispatchers|AssignOnDeath _bp_health (delegate Custom|OnDeath_Event))
  (EventDispatchers|BindEventtoOnDamage _bp_health (delegate Custom|OnDamage_Event))
  (bind _out (Default|GetNormalizedHealth (Variables|Default|GetBP_Health)))
  (Class|BPIUI|AdjustHealth(Message) (UserInterface|GetWidget (Variables|Default|GetWidget)) _out)
  (CallFunction|ChildBeginPlay))

(fn ConstructionScript)

(fn GiveLife
  (params (Give :type Float%20%28double-precision%29))
  (bind _newhealth (Default|ApplyDamage (Variables|Default|GetBP_Health) (* Give -1.0)))
  (Development|PrintString "Wow" true true "(R=0.468323,G=1.000000,B=0.407714,A=1.000000)")
  (Niagara|SpawnSystematLocation "/Game/Main/VFX/Main/HealthGrenade/NS_HealthGrenadeEned.NS_HealthGrenadeEned" (Transformation|GetWorldLocation (Variables|Default|GetStaticMesh)))
  (return _newhealth))

(fn TakeLife
  (params (Take :type Float%20%28double-precision%29))
  (bind _newhealth (Default|ApplyDamage (Variables|Default|GetBP_Health) Take))
  (Development|PrintString "Ow" true true "(R=1.000000,G=0.168231,B=0.474153,A=1.000000)")
  (return _newhealth))